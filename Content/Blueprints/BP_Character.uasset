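; Character Blueprint that turns the actor in yaw with the A (left) and D (right) keys.
; Each key plays its own timeline, which drives a per-tick Degrees value that Tick adds to the actor's yaw while either turn is active.
; Pressing a key during the opposite turn reverses that timeline instead of starting a new one, and a finished timeline zeroes Degrees.
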(event Custom|TurnCharacter
  (bind _returnvalue (Transformation|GetActorRotation))
  ;[1 1 1] Turns character by the amount of degrees
  (Transformation|SetActorRotation (Math|Rotator|MakeRotator (.roll _returnvalue) (.pitch _returnvalue) (+ (.yaw _returnvalue) (Variables|Default|GetDegrees)))))

(event Custom|ShouldTurn
  ;[1 1 1] Checks if the character should turn or not
  (if (not (and (Variables|Default|GetAFinished) (Variables|Default|GetDFinished)))
    (CallFunction|TurnCharacter)))

(event EventBeginPlay)

(event Collision|EventActorBeginOverlap
  (params (OtherActor :type Actor%20Object%20Reference)))

(event EventTick
  (params (DeltaSeconds :type Float%20%28single-precision%29))
  (CallFunction|ShouldTurn))

(event Input|KeyboardEvents|D
  (params (Key :type Key%20Structure :default "AnyKey"))
  ;[1 1 1] Turn Right and reverse if the Turn Left is still playing
  (:Pressed
    (if (Variables|Default|GetAFinished)
      (Variables|Default|SetDFinished false)
      (bind _charrot (Timeline|CharRotationRight PlayFromStart)
        (:Update
          (Variables|Default|SetDegrees _charrot))
        (:Finished
          (Variables|Default|SetDFinished true)
          (Variables|Default|SetDegrees 0.0)))
      (else
        ;[1 1 1] Turn Left and reverse if the Turn Right is still playing
        (bind _charrot_2 (Timeline|CharRotationLeft Reverse)
          (:Update
            (Variables|Default|SetDegrees _charrot_2))
          (:Finished
            (Variables|Default|SetAFinished true)
            (Variables|Default|SetDegrees 0.0)))))))

(event Input|KeyboardEvents|A
  (params (Key :type Key%20Structure :default "AnyKey"))
  ;[1 1 1] Turn Left and reverse if the Turn Right is still playing
  (:Pressed
    (if (Variables|Default|GetDFinished)
      (Variables|Default|SetAFinished false)
      (bind _charrot (Timeline|CharRotationLeft PlayFromStart)
        (:Update
          (Variables|Default|SetDegrees _charrot))
        (:Finished
          (Variables|Default|SetAFinished true)
          (Variables|Default|SetDegrees 0.0)))
      (else
        ;[1 1 1] Turn Right and reverse if the Turn Left is still playing
        (bind _charrot_2 (Timeline|CharRotationRight Reverse)
          (:Update
            (Variables|Default|SetDegrees _charrot_2))
          (:Finished
            (Variables|Default|SetDFinished true)
            (Variables|Default|SetDegrees 0.0)))))))

(fn ConstructionScript)